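; Central game logic for an arcade game where button sequences kill approaching enemies, managing targeting, spawning, lives and high score.
; Tick highlights the closest living enemy as target, and widget input is checked against its sequence, resetting on mistakes.
; Completed sequences fire a homing shot and spawn a replacement whose speed scales with kills.
; KillZone overlaps cost lives with timeline-animated HUD feedback, saving the local high score at game over.
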(event OnComponentBeginOverlap(KillZone)
  (params (OverlappedComponent :type Primitive%20Component%20Object%20Reference) (OtherActor :type Actor%20Object%20Reference) (OtherComp :type Primitive%20Component%20Object%20Reference) (OtherBodyIndex :type Integer) (bFromSweep :type Boolean) (SweepResult :type Hit%20Result%20Structure%20%28by%20ref%29))
  (bind _gamewindow (Variables|Default|GetGameWindow))
  (Utilities|Casting|CastToBP_EnemyDefault OtherActor)
  (bind _result (Math|Integer|DecrementInt (Variables|Default|GetLives))
    (:%20%20
      (CallFunction|LoseLife)
      (if (== _result 0)
        ;[1 1 1] Game over
        (CallFunction|SaveGame)
        (bind _asbp_saver (Utilities|Casting|CastToBP_Saver (Variables|Default|GetSavSubClass)))
        (Variables|/Game/Blueprints/Widgets/BPW_GameWindow.BPW_GameWindow_C|SetHighScore _gamewindow (Variables|/Game/Blueprints/Logic/BP_Saver.BP_Saver_C|GetHighScore _asbp_saver))
        (Variables|/Game/Blueprints/Widgets/BPW_GameWindow.BPW_GameWindow_C|SetGameOver _gamewindow true)
        (else
          (Utilities|Casting|CastToBP_EnemyDefault OtherActor)
          (CallFunction|OffScreenKillandRespawn))))))

(event Custom|IncomingSequence
  (params (InputSequence :type Enum_SequenceItem%20Enum :default "NewEnumerator0"))
  (bind _gamewindow (Variables|Default|GetGameWindow))
  ;[1 1 1] Compare current sequence to enemies, if we find a matching enemy (closest to player) keep going otherwise reset sequence
  (bind _returnvalue (Utilities|Array|Add (Variables|Default|GetCurrentSequence) InputSequence))
  (if (Utilities|Enum|Equal(Enum) (Utilities|Array|Get(acopy) (Variables|/Game/Blueprints/Enemies/BP_EnemyDefault.BP_EnemyDefault_C|GetMySequence (Variables|Default|GetTargetEnemy)) _returnvalue) InputSequence)
    (Default|IncSeqTrack (Variables|Default|GetTargetEnemy))
    (if (== (- (Utilities|Array|Length (Variables|/Game/Blueprints/Enemies/BP_EnemyDefault.BP_EnemyDefault_C|GetMySequence (Variables|Default|GetTargetEnemy))) 1) _returnvalue)
      (CallFunction|KillandRespawn (Variables|Default|GetTargetEnemy))
      (bind _output_get (Variables|/Game/Blueprints/Widgets/BPW_GameWindow.BPW_GameWindow_C|SetKillCount _gamewindow (+ (Variables|/Game/Blueprints/Widgets/BPW_GameWindow.BPW_GameWindow_C|GetKillCount _gamewindow) 1)))
      (Variables|Default|SetKillCountLocal _output_get))
    (else
      (CallFunction|Incorrect))))

(event Custom|Reset%20Sequence
  (Utilities|Array|Clear (Variables|Default|GetCurrentSequence))
  (Default|ResetSeqTrack (Variables|Default|GetTargetEnemy)))

(event Custom|SaveGame
  ;[1 1 1] Save game and store high score to leaderboard
  (bind _asbp_saver (Utilities|Casting|CastToBP_Saver (Variables|Default|GetSavSubClass)))
  (if (> (Variables|Default|GetKillCountLocal) (Variables|/Game/Blueprints/Logic/BP_Saver.BP_Saver_C|GetHighScore _asbp_saver))
    (Variables|/Game/Blueprints/Logic/BP_Saver.BP_Saver_C|SetHighScore _asbp_saver (Variables|Default|GetKillCountLocal)))
  (SaveGame|SaveGametoSlot (Variables|Default|GetSavSubClass) "highscoreLocal"))

(event Custom|DEBUG%20SPAWN%20NEW
  ;[1 1 1] Debug Spawning, probably move to it's own blueprint?
  (bind _returnvalue (Game|SpawnActorfromClass (|SelectionProcess) (Math|Transform|MakeTransform (Math|Vector|MakeVector (Math|Random|RandomFloatinRange -1.8e+02 1.8e+02) -412.0 0.0) "0, 0, 0" "1,1,1") "Undefined" 0 0))
  (Variables|/Game/Blueprints/Enemies/BP_EnemyDefault.BP_EnemyDefault_C|SetSpeedMulti (.AsBP%20Enemy%20Default (Utilities|Casting|CastToBP_EnemyDefault _returnvalue)) (+ (/ (Math|Conversions|ToFloat(Integer) (Variables|Default|GetKillCountLocal)) 7.0) 1.0))
  (Variables|/Game/Blueprints/Enemies/BP_EnemyDefault.BP_EnemyDefault_C|SetLogicBP (.AsBP%20Enemy%20Default (Utilities|Casting|CastToBP_EnemyDefault _returnvalue)) self))

(event Custom|OffScreenKillAndRespawn
  ;[1 1 1] Death Handling for Enemies
  (Actor|DestroyActor (Variables|Default|GetTargetEnemy))
  (CallFunction|DEBUGSPAWNNEW)
  (CallFunction|ResetDistCheck))

(event Custom|Incorrect
  (CallFunction|ResetSequence)
  (Default|Incorrect (Variables|Default|GetTargetEnemy)))

(event Custom|LoseLife
  (bind _gamewindow (Variables|Default|GetGameWindow))
  (bind _bpw_hearts (Variables|/Game/Blueprints/Widgets/BPW_GameWindow.BPW_GameWindow_C|GetBPW_Hearts _gamewindow))
  ;[1 1 1] Lose Life
  (Utilities|FlowControl|Sequence
    (:then_0
      (bind _output_get (Variables|/Game/Blueprints/Widgets/BPW_Hearts.BPW_Hearts_C|SetLives _bpw_hearts (Variables|Default|GetLives)))
      (bind _alpha (Timeline|ReduceHearts PlayFromStart)
        (:Update
          (Variables|/Game/Blueprints/Widgets/BPW_Hearts.BPW_Hearts_C|SetLivesAlpha _bpw_hearts (Math|Float|Lerp (Utilities|Select :Index _output_get :Option%200 0.33 :Option%201 0.66 :Option%202 1.0 :Option%203 1.0) (Utilities|Select :Index _output_get :Option%200 0.0 :Option%201 0.33 :Option%202 0.66 :Option%203 1.0) _alpha)))))
    (:then_1
      (bind _alpha_2 (Timeline|Timeline_0 PlayFromStart)
        (:Update
          (Variables|/Game/Blueprints/Widgets/BPW_GameWindow.BPW_GameWindow_C|SetHurtAlpha _gamewindow _alpha_2))))))

(event Custom|KillAndRespawn
  (params (EnemyToKill :type BP%20Enemy%20Default%20Object%20Reference))
  ;[1 1 1] Death Handling for Enemies
  (bind _returnvalue (Game|SpawnActorfromClass "/Game/Blueprints/Logic/BP_ParticleShot.BP_ParticleShot_C" (Math|Transform|MakeTransform "0.000000,300.000000,30.000000" (Math|Rotator|MakeRotator 0.0 0.0 (Math|Random|RandomFloatinRange -9e+01 9e+01))) "Undefined" 0 0))
  (Default|HomingSetup _returnvalue (Variables|Default|GetTargetEnemy) (Utilities|Array|Get(acopy) (Variables|/Game/Blueprints/Enemies/BP_EnemyDefault.BP_EnemyDefault_C|GetMySequence (Variables|Default|GetTargetEnemy)) (Utilities|Array|LastIndex (Variables|/Game/Blueprints/Enemies/BP_EnemyDefault.BP_EnemyDefault_C|GetMySequence (Variables|Default|GetTargetEnemy)))))
  (Utilities|Array|Add (Variables|Default|GetDyingEnemies) (Variables|Default|GetTargetEnemy))
  (Variables|/Game/Blueprints/Enemies/BP_EnemyDefault.BP_EnemyDefault_C|SetIsDead (Variables|Default|GetTargetEnemy) true)
  (CallFunction|ResetSequence)
  (Variables|Default|SetTargetEnemy 0)
  (CallFunction|DEBUGSPAWNNEW)
  (CallFunction|ResetDistCheck))

(event EventBeginPlay
  (bind _returnvalue (Game|GetPlayerController 0))
  ;[1 1 1] Load Local Leaderboard
  (bind _returnvalue_2 (SaveGame|DoesSaveGameExist "highscoreLocal"))
  (if _returnvalue_2
    (bind _returnvalue_3 (SaveGame|LoadGamefromSlot "highscoreLocal"))
    (Variables|Default|SetSavSubClass _returnvalue_3)
    (else
      (bind _returnvalue_4 (SaveGame|CreateSaveGameObject "/Game/Blueprints/Logic/BP_Saver.BP_Saver_C"))
      (Variables|Default|SetSavSubClass _returnvalue_4)))
  ;[1 1 1] Enable UI for buttons
  (Variables|/Script/Engine.PlayerController|SetbShowMouseCursor _returnvalue true)
  (bind _returnvalue_5 (UserInterface|CreateWidget "/Game/Blueprints/Widgets/BPW_GameWindow.BPW_GameWindow_C" _returnvalue))
  (bind _output_get (Variables|Default|SetGameWindow _returnvalue_5))
  (Variables|Default|SetButtons (Variables|/Game/Blueprints/Widgets/BPW_GameWindow.BPW_GameWindow_C|GetBPW_Buttons _output_get))
  (UserInterface|Viewport|AddtoViewport (Variables|Default|GetGameWindow) 0)
  (EventDispatchers|BindEventtoInputRecieved (Variables|Default|GetButtons) (delegate Custom|IncomingSequence))
  (CallFunction|ResetDistCheck))

(event EventTick
  (params (DeltaSeconds :type Float%20%28single-precision%29))
  (|FindClosestEnemy))

(fn ConstructionScript)

(event Custom|ResetDistCheck
  (params (DestroyedActor :type Actor%20Object%20Reference))
  (Variables|Default|SetClosestDistTemp 1e+05))