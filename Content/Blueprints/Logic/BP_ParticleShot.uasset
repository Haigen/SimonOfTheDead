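; BP_ParticleShot is a spinning sprite projectile, showing the last-pressed button, that flies at a target enemy and destroys it.
; HomingSetup picks the sprite, sets the homing target and captures 2D Bezier control points once, destroying itself if the target is invalid.
; The AlphaMovement timeline moves it along that cubic curve at fixed Z.
; Tick spins it and, within range, spawns an explosion and destroys both enemy and shot.
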(event Custom|HomingSetup
  (params (Target :type BP%20Enemy%20Default%20Object%20Reference) (LastPress :type Enum_SequenceItem%20Enum :default "NewEnumerator0"))
  (bind _homingloc (Variables|/Game/Blueprints/Enemies/BP_EnemyDefault.BP_EnemyDefault_C|GetHomingLoc Target))
  (bind _targetoffsetx (Variables|Default|GetTargetOffsetX))
  (bind _defaultsceneroot (Variables|Default|GetDefaultSceneRoot))
  (bind _returnvalue (Transformation|GetWorldLocation _homingloc))
  (bind _returnvalue_2 (Transformation|GetWorldLocation _defaultsceneroot))
  (bind (_x _y) (Math|Vector|BreakVector _returnvalue))
  (bind (_x_2 _y_2) (Math|Vector|BreakVector _returnvalue_2))
  (bind _returnvalue_3 (* _x _targetoffsetx))
  (bind _returnvalue_4 (Math|Vector2D|MakeVector2D _returnvalue_3 _y))
  (Rendering|Components|Sprite|SetSprite (Variables|Default|GetPaperSprite) (Utilities|Select :Index LastPress :NewEnumerator0 "/Game/Textures/UI/Button_A1_Sprite.Button_A1_Sprite" :NewEnumerator1 "/Game/Textures/UI/Button_A2_Sprite.Button_A2_Sprite" :NewEnumerator2 "/Game/Textures/UI/Button_A3_Sprite.Button_A3_Sprite" :NewEnumerator3 "/Game/Textures/UI/Button_A4_Sprite.Button_A4_Sprite" :NewEnumerator4 0 :NewEnumerator7 0 :NewEnumerator5 0 :NewEnumerator6 0))
  (Variables|Default|SetTargetEnemy Target)
  (Utilities|IsValid _homingloc
    (:Is%20Valid
      (Variables|/Script/Engine.ProjectileMovementComponent|SetHomingTargetComponent (Variables|Default|GetProjectileMovement) _homingloc)
      (Variables|Default|SetHomeLoc (Math|Vector2D|MakeVector2D _x_2 _y_2))
      (Variables|Default|SetTargetLoc (Math|Vector2D|MakeVector2D _x _y))
      (Variables|Default|SetTargetOffsetLoc _returnvalue_4)
      (Variables|Default|SetHomeOffsetLoc (Math|Vector2D|MakeVector2D (.X (Math|Vector2D|BreakVector2D _returnvalue_4)) _y_2))
      (bind _alpha (Timeline|AlphaMovement PlayFromStart)
        (:Update
          (bind _location (CallFunction|GetPointonBezierCurve (Variables|Default|GetHomeLoc) (Variables|Default|GetHomeOffsetLoc) (Variables|Default|GetTargetOffsetLoc) (Variables|Default|GetTargetLoc) _alpha))
          (Transformation|SetActorLocation (Math|Conversions|ToVector(Vector2D) _location 1e+01) false false))))
    (:Is%20Not%20Valid
      (Actor|DestroyActor))))

(event Collision|EventActorBeginOverlap
  (params (OtherActor :type Actor%20Object%20Reference)))

(event EventTick
  (params (DeltaSeconds :type Float%20%28single-precision%29))
  (Transformation|AddLocalRotation (Variables|Default|GetPaperSprite) "50.000000,0.000000,0.000000" false false)
  (if (< (Transformation|GetDistanceTo (Components|GetOwner (Variables|/Script/Engine.ProjectileMovementComponent|GetHomingTargetComponent (Variables|Default|GetProjectileMovement)))) 5e+01)
    (Effects|SpawnEmitteratLocation "/Game/Particles/P_Explosion.P_Explosion" (Transformation|GetActorLocation (Variables|Default|GetTargetEnemy)))
    (Default|DestroyEnemyActor (Variables|Default|GetTargetEnemy))
    (Actor|DestroyActor)))

(fn ConstructionScript)

(fn GetPointonBezierCurve
  (params (Home :type Vector%202D%20Structure) (HomeOffset :type Vector%202D%20Structure) (TargetOffset :type Vector%202D%20Structure) (Target :type Vector%202D%20Structure) (t :type Float%20%28single-precision%29))
  (LocalVariables|Setu (- 1.0 t))
  (LocalVariables|Sett2 (* t t))
  (LocalVariables|Setu2 (* (LocalVariables|Getu) (LocalVariables|Getu)))
  (LocalVariables|Setu3 (* (LocalVariables|Getu2) (LocalVariables|Getu)))
  (LocalVariables|Sett3 (* (LocalVariables|Gett2) t))
  (bind _output_get (LocalVariables|SetResult (+ (* Home (LocalVariables|Getu3)) (* HomeOffset (* 3.0 (LocalVariables|Getu2) t)) (* TargetOffset (* 3.0 (LocalVariables|Getu) (LocalVariables|Gett2))) (* Target (LocalVariables|Gett3)))))
  (return _output_get))