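; BP_SequenceController turns keyboard input into sequence inputs for the game logic.
; On BeginPlay it finds the first BP_GameLogic actor in the level and caches a reference to it.
; Each arrow key calls IncomingSequence on that actor with its own direction enum value.
; The R key restarts play by opening the Testmap_01 level by name.
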(event EventBeginPlay
  (bind _outactors (Actor|GetAllActorsOfClass "/Game/Blueprints/Logic/BP_GameLogic.BP_GameLogic_C"))
  (Variables|Default|SetGameLogicBP (Utilities|Array|Get(acopy) _outactors)))

(event EventTick
  (params (DeltaSeconds :type Float%20%28single-precision%29)))

(event Input|KeyboardEvents|Left
  (params (Key :type Key%20Structure))
  (:Pressed
    (Default|IncomingSequence (Variables|Default|GetGameLogicBP) "NewEnumerator3")))

(event Input|KeyboardEvents|Right
  (params (Key :type Key%20Structure))
  (:Pressed
    (Default|IncomingSequence (Variables|Default|GetGameLogicBP) "NewEnumerator1")))

(event Input|KeyboardEvents|Up
  (params (Key :type Key%20Structure))
  (:Pressed
    (Default|IncomingSequence (Variables|Default|GetGameLogicBP) "NewEnumerator0")))

(event Input|KeyboardEvents|Down
  (params (Key :type Key%20Structure))
  (:Pressed
    (Default|IncomingSequence (Variables|Default|GetGameLogicBP) "NewEnumerator2")))

(event Input|KeyboardEvents|R
  (params (Key :type Key%20Structure))
  (:Pressed
    (Game|OpenLevel(byName) "Testmap_01")))

(fn ConstructionScript)