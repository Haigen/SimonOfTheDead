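; Base zombie enemy that shows a random five-button sequence as sprites and walks toward a goal.
; BeginPlay picks its look, sequence and a side waypoint that avoids the buttons; Tick drives AI movement via that waypoint to the central goal, or destroys it when IsDead.
; Events advance, reset or red-flash the sequence on error, then refresh the current step's scale and brightness highlight if the enemy is targeted.
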(event Custom|ResetSeqTrack
  ;[1 1 1] seq track mgmnt
  (Variables|Default|SetSeqTrack 0)
  (CallFunction|SetHighlight))

(event Custom|IncSeqTrack
  ;[1 1 1] seq track mgmnt
  (Math|Integer|IncrementInt (Variables|Default|GetSeqTrack)
    (:%20%20
      (CallFunction|SetHighlight))))

(event Custom|Incorrect
  ;[1 1 1] seq track mgmnt
  (|SetColourRedFlash)
  (CallFunction|SetHighlight))

(event Custom|SetHighlight
  ;[1 1 1] Set highlighted seq
  (if (Variables|Default|GetIsTarget)
    (Utilities|FlowControl|Sequence
      (:then_0
        (|SetOn/Off))
      (:then_1
        (|SetScale)
        (|SetColour)))))

(event EventBeginPlay
  ;[1 1 1] Randomly choose enemy sprite
  (Sprite|SetFlipbook (Variables|Default|GetMainEnemySprite) (Utilities|Select :Index (Math|Random|RandomIntegerinRange 0 2) :Option%200 "/Game/Textures/Monsters/FB_Zombie01.FB_Zombie01" :Option%201 "/Game/Textures/Monsters/FB_Zombie02.FB_Zombie02" :Option%202 "/Game/Textures/Monsters/FB_Zombie03.FB_Zombie03"))
  ;[1 1 1] Are we left or right side? Sets waypoint to move to in order to avoid buttons
  (Variables|Default|SetDestination (select (>= (.x (Transformation|GetActorLocation)) 0.0) "200.000000,270.000000,0.000000" "-200.000000,270.000000, 0"))
  ;[1 1 1] Randomly generate a pattern
  (for _index (range 0 4)
    (Utilities|Array|Add (Variables|Default|GetMySequence) (Utilities|Select :Index (Math|Random|RandomIntegerinRange 0 3) :Option%200 "NewEnumerator0" :Option%201 "NewEnumerator1" :Option%202 "NewEnumerator2" :Option%203 "NewEnumerator3"))
    (Utilities|Array|Add (Variables|Default|GetPanels) false))
  (for (_array_element _array_index) (Variables|Default|GetMySequence)
    (Rendering|Components|Sprite|SetSprite (.Target (|SpriteSelection _array_element _array_index)) (.NewSprite (|SpriteSelection _array_element _array_index)))
    (CallFunction|SetHighlight)))

(event Collision|EventActorBeginOverlap
  (params (OtherActor :type Actor%20Object%20Reference)))

(event EventTick
  (params (DeltaSeconds :type Float%20%28single-precision%29))
  ;[1 1 1] Are we the dead?
  (if (Variables|Default|GetIsDead)
    ;[1 1 1] Run death anim (juice it up later)
    (Actor|DestroyActor)
    (else
      ;[1 1 1] Walk towards goal
      (|WalkingLogic))))

(fn ConstructionScript)