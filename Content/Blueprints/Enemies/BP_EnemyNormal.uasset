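; BP_EnemyNormal is the normal enemy Blueprint, a child class that displays a main sprite and a sequence across five panels.
; On BeginPlay it calls SetMainSprite, SetupPanels and SetSequence in that order.
; SetupPanels adds the Sequence01 to Sequence05 references to the SpritePanels array before SetSequence runs.
; SetMainSprite and SetSequence are defined outside this graph, and the construction script only calls the parent's.
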(event Collision|EventActorBeginOverlap
  (params (OtherActor :type Actor%20Object%20Reference)))

(event EventTick
  (params (DeltaSeconds :type Float%20%28single-precision%29)))

(event EventSetupPanels
  (bind _spritepanels (Variables|Default|GetSpritePanels))
  (Utilities|Array|Add _spritepanels (Variables|Default|GetSequence01))
  (Utilities|Array|Add _spritepanels (Variables|Default|GetSequence02))
  (Utilities|Array|Add _spritepanels (Variables|Default|GetSequence03))
  (Utilities|Array|Add _spritepanels (Variables|Default|GetSequence04))
  (Utilities|Array|Add _spritepanels (Variables|Default|GetSequence05)))

(event EventBeginPlay
  (CallFunction|SetMainSprite)
  (CallFunction|SetupPanels)
  (CallFunction|SetSequence))

(fn ConstructionScript
  (|CallParentFunction))