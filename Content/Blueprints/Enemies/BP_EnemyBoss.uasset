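; Boss enemy that shows a random five-button sequence on sprite panels, repeated to make ten steps.
; BeginPlay builds the sequence; while the boss is targeted, the current panel is enlarged and brightened, wrapping for the second pass.
; Advancing the track clears shield sprites one by one.
; An incorrect input flashes red and restores shields, as does losing target status, while a separate event resets the track.
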(event Custom|SetShields
  (params (ResetShields :type Boolean))
  (bind _seqshields (Variables|Default|GetSeqShields))
  ;[1 1 1] Set Shields
  (if ResetShields
    (for (_ _array_index) _seqshields
      (Utilities|Array|SetArrayElem _seqshields _array_index true))
    (else
      (Utilities|Array|SetArrayElem (Variables|Default|GetSeqShields) (- (Variables|Default|GetSeqTrack) 1) false)))
  (for _index (range 0 4)
    (Rendering|Components|Sprite|SetSprite (Utilities|Array|Get(acopy) (Variables|Default|GetSpritePanels) _index) (|ShieldSpriteSwap _index))))

(event EventBeginPlay
  (CallFunction|SetMainSprite)
  (CallFunction|SetupPanels)
  (CallFunction|SetSequence))

(event Collision|EventActorBeginOverlap
  (params (OtherActor :type Actor%20Object%20Reference)))

(event EventSetupPanels
  (bind _spritepanels (Variables|Default|GetSpritePanels))
  (Utilities|Array|Add _spritepanels (Variables|Default|GetPaperSprite))
  (Utilities|Array|Add _spritepanels (Variables|Default|GetPaperSprite1))
  (Utilities|Array|Add _spritepanels (Variables|Default|GetPaperSprite2))
  (Utilities|Array|Add _spritepanels (Variables|Default|GetPaperSprite3))
  (Utilities|Array|Add _spritepanels (Variables|Default|GetPaperSprite4)))

(event EventTick
  (params (DeltaSeconds :type Float%20%28single-precision%29)))

(event EventSetSequence
  (bind _mysequence (Variables|Default|GetMySequence))
  ;[1 1 1] Set Sequence
  (for _index (range 0 4)
    (Utilities|Array|Add (Variables|Default|GetMySequence) (Utilities|Select :Index (Math|Random|RandomIntegerinRange 0 3) :Option%200 "NewEnumerator0" :Option%201 "NewEnumerator1" :Option%202 "NewEnumerator2" :Option%203 "NewEnumerator3"))
    (Utilities|Array|Add (Variables|Default|GetActivePanels) false)
    (Utilities|Array|Add (Variables|Default|GetSeqShields) true))
  (for (_array_element _array_index) (Variables|Default|GetMySequence)
    (Rendering|Components|Sprite|SetSprite (.Target (|SpriteSelection_2 _array_element _array_index)) (.NewSprite (|SpriteSelection_2 _array_element _array_index))))
  (for _index_2 (range 0 4)
    (Utilities|Array|Add _mysequence (Utilities|Array|Get(acopy) _mysequence _index_2)))
  (CallFunction|SetHighlight))

(event EventIncorrect
  ;[1 1 1] Sequence Track Handling
  (|SetColourRedFlash_2)
  (CallFunction|SetShields true)
  (CallFunction|SetHighlight))

(event EventResetSeqTrack
  ;[1 1 1] Sequence Track Handling
  (Variables|Default|SetSeqTrack 0)
  (CallFunction|SetHighlight))

(event EventSetHighlight
  ;[1 1 1] Set Highlight/Scale/Colour
  (if (Variables|Default|GetIsTarget)
    (Utilities|FlowControl|Sequence
      (:then_0
        (|SetOn/Off_2))
      (:then_1
        (|SetScale_2 :!label _label)
        (|SetColour_2)))
    (else
      (CallFunction|SetShields true)
      (|SetOff_2)
      (goto _label))))

(event EventIncSeqTrack
  ;[1 1 1] Sequence Track Handling
  (Math|Integer|IncrementInt (Variables|Default|GetSeqTrack)
    (:%20%20
      (CallFunction|SetShields false)
      (CallFunction|SetHighlight))))

(fn ConstructionScript
  (|CallParentFunction))