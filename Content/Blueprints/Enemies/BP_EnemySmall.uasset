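; Small enemy Blueprint that supplies its idle flipbook and three sequence panel sprites to logic inherited from its parent.
; SetMainSprite assigns the flipbook, and SetupPanels fills the SpritePanels array.
; On BeginPlay a timeline drives panel alpha, tinting active panels white and inactive ones dark grey.
; Tick continually sets Timeline0's play rate from SpeedMulti.
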(event EventBeginPlay
  (|CallParentFunction)
  (bind _alpha (Timeline|Timeline_0 PlayFromStart)
    (:Update
      (for (_array_element _array_index) (Variables|Default|GetActivePanels)
        (Sprite|SetSpriteColor (Utilities|Array|Get(acopy) (Variables|Default|GetSpritePanels) _array_index) (select _array_element (Utilities|Struct|MakeLinearColor 1.0 1.0 1.0 _alpha) (Utilities|Struct|MakeLinearColor 0.33 0.33 0.33 _alpha)))))))

(event Collision|EventActorBeginOverlap
  (params (OtherActor :type Actor%20Object%20Reference))
  (|CallParentFunction OtherActor) ; This node is disabled and will not be called.\nDrag off pins to build functionality.
)

(event EventTick
  (params (DeltaSeconds :type Float%20%28single-precision%29))
  (|CallParentFunction DeltaSeconds)
  (Components|Timeline|SetPlayRate (Variables|Default|GetTimeline_0) (Variables|Default|GetSpeedMulti)))

(event EventSetupPanels
  (bind _spritepanels (Variables|Default|GetSpritePanels))
  (Utilities|Array|Add _spritepanels (Variables|Default|GetSequence01))
  (Utilities|Array|Add _spritepanels (Variables|Default|GetSequence02))
  (Utilities|Array|Add _spritepanels (Variables|Default|GetSequence03)))

(event EventSetMainSprite
  (Sprite|SetFlipbook (Variables|Default|GetMainEnemySprite) "/Game/2DPlatformingKit/Sprites/Enemies/Flipbooks/Enemy_idle.Enemy_idle"))

(fn ConstructionScript
  (|CallParentFunction))