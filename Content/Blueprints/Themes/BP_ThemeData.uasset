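; BP_ThemeData holds a theme's button graphics for the world and UI, with variants for colour blind settings.
; UpdateButtonGraphics picks the Original, Protan, Deuteran or Tritan button set for each from ColourBlindSetting.
; SetGraphics writes that set's Top, Right, Bottom and Left entries into the theme arrays by index.
; It then calls UpdateEnemyGraphicsSet, which is empty here.
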(event Custom|UpdateButtonGraphics
  (bind _colourblindoptions (Variables|Default|GetColourBlindOptions))
  (bind _colourblindoptions_ui (Variables|Default|GetColourBlindOptions_UI))
  (bind (_default _protan _deuteran _tritan) (Utilities|Struct|BreakButtons_ColourBlindOptions _colourblindoptions))
  (bind (_default_2 _protan_2 _deuteran_2 _tritan_2) (Utilities|Struct|BreakButtons_ColourBlindOptions _colourblindoptions_ui))
  (bind _output_get (Variables|Default|SetCurrentButtonSet_UI (Utilities|Select :Index (Variables|Default|GetColourBlindSetting) :NewEnumerator0 _default_2 :NewEnumerator1 _protan_2 :NewEnumerator2 _deuteran_2 :NewEnumerator3 _tritan_2)))
  (CallFunction|SetGraphics (Variables|Default|GetTheme_SetButtons_UI) _output_get) ; UI
  (bind _output_get_2 (Variables|Default|SetCurrentButtonSet (Utilities|Select :Index (Variables|Default|GetColourBlindSetting) :NewEnumerator0 _default :NewEnumerator1 _protan :NewEnumerator2 _deuteran :NewEnumerator3 _tritan)))
  (CallFunction|SetGraphics (Variables|Default|GetTheme_SetButtons) _output_get_2)
  (CallFunction|UpdateEnemyGraphicsSet))

(event Custom|UpdateEnemyGraphicsSet)

(event EventBeginPlay)

(event Collision|EventActorBeginOverlap
  (params (OtherActor :type Actor%20Object%20Reference)))

(event EventTick
  (params (DeltaSeconds :type Float%20%28single-precision%29)))

(fn ConstructionScript)

(fn SetGraphics
  (params (ThemeSet :type Array%20of%20Paper%20Sprite%20Object%20References) (ButtonSet :type Buttons%20Default%20Structure))
  (bind (_top _right _bottom _left) (Utilities|Struct|BreakButtons_Default ButtonSet))
  (for (_ _array_index) ThemeSet
    (Utilities|Array|SetArrayElem ThemeSet _array_index (Utilities|Select :Index _array_index :Option%200 _top :Option%201 _right :Option%202 _bottom :Option%203 _left))))